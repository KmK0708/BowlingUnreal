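; Bowling pin actor that can be hidden once knocked over and reset to its starting position.
; Shortly after BeginPlay it stores its transform as the reset point.
; HideThePin turns off mesh physics and moves the actor to a fixed off-lane location.
; Reset disables physics, teleports both the actor and its mesh component to the stored transform, then re-enables simulation.
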(event `self.ReceiveBeginPlay`
  ;[1 1 1] Delay and store the starting transform for resetting
  (`KismetSystemLibrary.Delay` 0.2)
  (set `self.ResetTransform` (`self.GetTransform`)))

(event `HideThePin`
  ;[1 1 1] If the pins been knocked over, turn off physics and hide it
  (`PrimitiveComponent.SetSimulatePhysics` (`self.StaticMeshComponent`) false)
  (`self.K2_SetActorLocation` (0.0 -500.0 0.0)))

(event `Reset`
  (bind _resettransform (`self.ResetTransform`))
  (bind _staticmeshcomponent (`self.StaticMeshComponent`))
  ;[1 1 1] Reset the pin
  (`PrimitiveComponent.SetSimulatePhysics` _staticmeshcomponent false)
  (`self.K2_SetActorTransform` _resettransform false true)
  (`SceneComponent.K2_SetWorldTransform` _staticmeshcomponent _resettransform false true)
  (`PrimitiveComponent.SetSimulatePhysics` _staticmeshcomponent true))

(fn `UserConstructionScript`)