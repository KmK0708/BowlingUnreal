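; Bowling game mode that judges each throw and resets the ball and pins.
; BeginPlay caches the gutter zone, checking zone and ball; Tick waits after the gutter zone flags InZone, then counts pins overlapping the checking zone.
; No pins left shows a strike animation, calls ResultGame and resets all pins; otherwise it shows a miss animation and hides fallen pins.
; Text helpers for remaining pins and throw count go uncalled here; throw-impulse logic is disconnected.
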(event `self.ReceiveBeginPlay`
  ;[1 1 1] 오브젝트 레퍼런스 불러오기
  (bind _returnvalue (`GameplayStatics.GetActorOfClass` "/Game/BP/BP_Gutterzone.BP_Gutterzone_C"))
  (set `self.GutterzoneRef` _returnvalue)
  (bind _returnvalue_2 (`GameplayStatics.GetActorOfClass` "/Game/BP/BP_Checkingzone.BP_Checkingzone_C"))
  (set `self.chekingZoneRef` _returnvalue_2)
  (bind _returnvalue_3 (`GameplayStatics.GetActorOfClass` "/Game/BP/BP_NewBowlingBall.BP_NewBowlingBall_C"))
  (set `self.NewBall` _returnvalue_3))

(event `self.ReceiveTick`
  (params (DeltaSeconds :type "Float (single-precision)"))
  (bind _widgetref (`/Game/BP/BP_NewBowlingBall.WidgetRef` (`self.NewBall`)))
  (bind _overlappingactors (`PrimitiveComponent.GetOverlappingActors` (`/Game/BP/BP_Checkingzone.Box` (`self.chekingZoneRef`)) "/Game/Blueprints/BowlingPin_BP.BowlingPin_BP_C"))
  (bind _alldowntext (`/Game/UMG/WBP_PlayWidget.AllDownText` _widgetref))
  ;[1 1 1] 세워져있는 볼링핀 체크 후 다 넘어지면 Strike UI 와 애니메이션 출력후 리셋하기
  ; 다 안넘어가면 넘어진 핀 숨기고 볼링공 리셋하기
  (if (`/Game/BP/BP_Gutterzone.InZone` (`self.GutterzoneRef`))
    (`KismetSystemLibrary.Delay` 4.0)
    (bind _outactors (`GameplayStatics.GetAllActorsOfClass` "/Game/Blueprints/BowlingPin_BP.BowlingPin_BP_C"))
    (if (== (`KismetArrayLibrary.Array_Length` _overlappingactors) 0)
      (`Widget.SetVisibility` _alldowntext "Visible")
      (`UserWidget.PlayAnimation` _widgetref (`/Game/UMG/WBP_PlayWidget.Strike` _widgetref) 0.0 1 "Forward" 1.0 false)
      (`KismetSystemLibrary.Delay` 2.0)
      (`Widget.SetVisibility` _alldowntext "Hidden")
      (`/Game/UMG/WBP_PlayWidget.ResultGame` _widgetref)
      (for _array_element _outactors
        (`/Game/Blueprints/BowlingPin_BP.Reset` _array_element))
      (`/Game/BP/BP_NewBowlingBall.ResetBall` (`self.NewBall`))
      (else
        ;[1 1 1] 다 안넘어지면 다시 리셋
        (`self.Hide Pin N Reset`)
        (`/Game/BP/BP_NewBowlingBall.ResetBall` (`self.NewBall`))
        (for _array_element_2 _outactors
          (if (== (`KismetArrayLibrary.Array_Find` _overlappingactors _array_element_2) -1)
            (`/Game/Blueprints/BowlingPin_BP.HideThePin` _array_element_2)))))))

(event `/Game/interface/BPI_Throw.Throw`
  (params (PressTime :type "Float (double-precision)")))

(fn `Hide Pin N Reset`
  (bind _widgetref (`/Game/BP/BP_NewBowlingBall.WidgetRef` (`self.NewBall`)))
  (`Widget.SetVisibility` (`/Game/UMG/WBP_PlayWidget.PinNotDown` _widgetref) "Visible")
  (`UserWidget.PlayAnimation` _widgetref (`/Game/UMG/WBP_PlayWidget.NotStrike` _widgetref) 0.0 1 "Forward" 1.0 false))

(fn `PinsNotDown`)

(fn `RemainPincheck`
  (`TextBlock.SetText` (`/Game/UMG/WBP_PlayWidget.RemainPinText` (`/Game/BP/BP_NewBowlingBall.WidgetRef` (`self.NewBall`))) (`KismetTextLibrary.Conv_StringToText` (`KismetStringLibrary.Concat_StrStr` "현재 남은 핀 : " (`KismetStringLibrary.Conv_IntToString` (`KismetArrayLibrary.Array_Length` (`PrimitiveComponent.GetOverlappingActors` (`/Game/BP/BP_Checkingzone.Box` (`self.chekingZoneRef`)) "/Game/Blueprints/BowlingPin_BP.BowlingPin_BP_C")))))))

(fn `ThrowTimeCheck`
  (bind _newball (`self.NewBall`))
  (`TextBlock.SetText` (`/Game/UMG/WBP_PlayWidget.ThrowtimeText` (`/Game/BP/BP_NewBowlingBall.WidgetRef` _newball)) (`KismetTextLibrary.Conv_StringToText` (`KismetStringLibrary.Concat_StrStr` "던진 횟수 : " (`KismetStringLibrary.Conv_IntToString` (`/Game/BP/BP_NewBowlingBall.ThrowTime` _newball))))))

(fn `UserConstructionScript`)