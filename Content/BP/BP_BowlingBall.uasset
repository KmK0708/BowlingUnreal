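; BP_BowlingBall is a physics-driven bowling ball actor that can be reset to its spawn transform.
; BeginPlay caches the transform; Reset restores it with physics briefly disabled and clears the bowled, caught and staging state.
; Tick shows the aim arrow while caught and a speed effect while the ball moves.
; Throw and mouse-wheel events are empty, leaving the impulse launch and yaw rotation logic disconnected.
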(event `self.ReceiveBeginPlay`
  ;[1 1 1] Spawn Transform resetting
  (set `self.ResetTransform` (`self.GetTransform`)))

(event `Reset`
  (bind _ball (`self.Ball`))
  ;[1 1 1] Reset Ball
  (`PrimitiveComponent.SetSimulatePhysics` _ball false)
  (`self.K2_SetActorTransform` (`self.ResetTransform`))
  (`PrimitiveComponent.SetSimulatePhysics` _ball true)
  (set `self.Bowled` false)
  (set `self.IsCatched?` false)
  (set `self.StagedLocation` (0.0 0.0 0.0)))

(event `Key|R`
  (params (Key :type "Key Structure")))

(event `InputAxisKey|MouseWheelAxis`
  (params (AxisValue :type "Float (single-precision)")))

(event `self.ReceiveTick`
  (params (DeltaSeconds :type "Float (single-precision)"))
  (`SceneComponent.SetHiddenInGame` (`self.ForwardArrow`) (not (`self.IsCatched?`)) false)
  (bind _returnvalue (`PrimitiveComponent.GetPhysicsLinearVelocity` (`self.Ball`) "None"))
  (`SceneComponent.SetHiddenInGame` (`self.SpeedEffect`) (== _returnvalue (0.0 0.0 0.0) :`ErrorTolerance` 50.0) false)
  (if (`self.Bowled`)
    _))

(event `/Game/interface/BPI_Throw.Throw`
  (params (PressTime :type "Float (double-precision)")))

(fn `UserConstructionScript`)