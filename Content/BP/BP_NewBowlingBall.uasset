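; BP_NewBowlingBall is a possessable bowling ball that the player slides sideways, aims with a mouse-wheel-rotated arrow, and throws.
; BeginPlay creates the play widget and saves the starting transform.
; Throw enables physics, applies an impulse along the arrow scaled by throwing power and the widget's press time, then possesses a newly spawned BP_MovePlayer at a fixed spot.
; ResetBall disables physics, restores the transform and arrow, and repossesses the ball.
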(event `InputAxis|MoveRight`
  (params (AxisValue :type "Float (single-precision)"))
  (`self.K2_SetActorLocation` (+ (* (* AxisValue (`self.MoveBall`)) (`self.GetActorRightVector`)) (`self.K2_GetActorLocation`))))

(event `InputAxisKey|MouseWheelAxis`
  (params (AxisValue :type "Float (single-precision)"))
  (`SceneComponent.K2_AddLocalRotation` (`self.Arrow`) (`KismetMathLibrary.MakeRotator` 0.0 0.0 AxisValue) false false))

(event `/Game/interface/BPI_Throw.Throw`
  (params (PressTime :type "Float (double-precision)"))
  (bind _ball (`self.Ball`))
  (bind _arrow (`self.Arrow`))
  ;[1 1 1] 버튼 누르는 시간 x 정해둔 파워 x 화살표가 향하는 방향으로  add impulse 해서 굴리기->정해둔 위치에 플레이어 스폰하고 포제스하기
  (`PrimitiveComponent.SetSimulatePhysics` _ball true)
  (`PrimitiveComponent.AddImpulse` _ball (* (`SceneComponent.GetForwardVector` _arrow) (`self.ThrowingPower`) (`/Game/UMG/WBP_PlayWidget.PressTime` (`self.WidgetRef`))) "None" false)
  (`SceneComponent.SetHiddenInGame` _arrow true false)
  (bind _returnvalue (`|SpawnActorFromClass` "/Game/BP/BP_MovePlayer.BP_MovePlayer_C" (`KismetMathLibrary.MakeTransform` (1610.0 -10.0 130.0) (struct :`Pitch` -30.0 :`Yaw` 180.0)) "Undefined" "MultiplyWithRoot" null null))
  (`Controller.Possess` (`GameplayStatics.GetPlayerController` 0) _returnvalue))

(event `ResetBall`
  ;[1 1 1] 공 원래 위치로-> 포제스 다시 공으로 가져오기
  (`PrimitiveComponent.SetSimulatePhysics` (`self.Ball`) false)
  (`self.K2_SetActorTransform` (`self.ResetTransform`))
  (`Controller.Possess` (`GameplayStatics.GetPlayerController` 0) self)
  (`SceneComponent.SetHiddenInGame` (`self.Arrow`) false false))

(event `self.ReceiveBeginPlay`
  ;[1 1 1] 시작 시, 위젯 생성 후 뷰포트
  ; 트랜스폼 설정
  (bind _returnvalue (`|CreateWidget` "/Game/UMG/WBP_PlayWidget.WBP_PlayWidget_C"))
  (bind _output_get (set `self.WidgetRef` _returnvalue))
  (`UserWidget.AddToViewport` _output_get 0)
  (set `self.ResetTransform` (`self.GetTransform`)))

(fn `UserConstructionScript`)